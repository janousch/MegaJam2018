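; Shared helper library for a horror game, giving one-call access to game-wide actions and key actors.
; Casts the game state to BP_GameState to reach the Wife and player, and to drive horror mode, post-process and blood.
; Wrappers toggle the Wife's chase and kill ability, control the player's flashlight and sound, and restart through BP_GameMode.
; Switching horror post-process also plays a matching transition or safe-transition cue through the player character.
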(fn GetBPGameState
  (return (.AsBP%20Game%20State (Utilities|Casting|CastToBP_GameState (Game|GetGameState)))))

(fn SetWifeChasing
  (params (IsChasing :type Boolean))
  (bind _asbp_game_state (CallFunction|GetBPGameState))
  (bind _wife (Variables|/Game/MegaJam/BP_GameState.BP_GameState_C|GetWife _asbp_game_state))
  (if IsChasing
    (Default|StartChasingPlayer _wife (Variables|/Game/MegaJam/BP_GameState.BP_GameState_C|GetPlayerCharacter _asbp_game_state))
    (else
      (Default|StopChasingPlayer _wife))))

(fn SetWifeCanKill
  (params (CanKill :type Boolean))
  (Variables|/Game/MegaJam/CrazyWifeBitch/BP_Wife.BP_Wife_C|SetCanKillPlayer (CallFunction|GetWife) CanKill))

(fn SetHorrorModeActive
  (params (IsActive :type Boolean) (HasToLerpPostProcess :type Boolean))
  (Default|SetHorrorModeActive (CallFunction|GetBPGameState) IsActive HasToLerpPostProcess))

(fn GetWife
  (return (Variables|/Game/MegaJam/BP_GameState.BP_GameState_C|GetWife (CallFunction|GetBPGameState))))

(fn GetPlayerCharacter
  (return (Variables|/Game/MegaJam/BP_GameState.BP_GameState_C|GetPlayerCharacter (CallFunction|GetBPGameState))))

(fn RestartGame
  (Default|Restart (CallFunction|GetBPGameMode)))

(fn GetBPGameMode
  (return (.AsBP%20Game%20Mode (Utilities|Casting|CastToBP_GameMode (Game|GetGameMode)))))

(fn SetHorrorPPActive
  (params (IsActive :type Boolean))
  (Default|SetHorrorPP (CallFunction|GetBPGameState) IsActive)
  (Sound|PlaySound (select IsActive "/Game/MegaJam/Sounds/transition_sfx_Cue.transition_sfx_Cue" "/Game/MegaJam/Sounds/safe_transition_sfx_Cue.safe_transition_sfx_Cue") 0 (CallFunction|TRANSITION)))

(fn SetBloodActive
  (params (IsActive :type Boolean))
  (Default|SetBloodActive (CallFunction|GetBPGameState) IsActive))

(fn SetFlashlightActive
  (params (IsActive :type Boolean))
  (Default|TurnFlashlightonOff (CallFunction|GetPlayerCharacter) IsActive))

(fn PlaySound
  (params (NewSound :type Sound%20Base%20Object%20Reference) (VolumeMultiplier :type Float%20%28single-precision%29))
  (Default|PlaySound (CallFunction|GetPlayerCharacter) NewSound VolumeMultiplier))

(fn StopSound
  (Default|StopSound (CallFunction|GetPlayerCharacter)))