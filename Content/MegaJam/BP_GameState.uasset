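; Game state that switches the level in and out of a horror mode, starting with it off.
; Shortly after BeginPlay it caches all blood decal and drop actors, which SetHorrorModeActive shows or hides while toggling player flashlight and audio.
; Pixel post-process and blood puddle are driven through material parameter collections, with timelines for optional fades.
; SetHorrorPP and SetBloodActive expose the post-process and blood parts separately.
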(event Custom|LerpPostProcess
  (if (Variables|Default|GetIsHorrorMordeActive?)
    (bind _newtrack_0 (Timeline|HorrorLerp Play)
      (:Update
        (Rendering|Material|SetScalarParameterValue "/Game/MegaJam/PostProcess/PC_Pixel.PC_Pixel" "Switch" _newtrack_0 :!class /Script/Engine.KismetMaterialLibrary)))
    (else
      (Timeline|HorrorLerp Reverse))))

(event Custom|SetBloodPuddleActive
  (params (IsActive :type Boolean))
  (if IsActive
    (bind _bloodtrack (Timeline|Timeline_0 Play)
      (:Update
        (Rendering|Material|SetScalarParameterValue "/Game/MegaJam/BloodDripping/PC_Blood.PC_Blood" "Blood" _bloodtrack :!class /Script/Engine.KismetMaterialLibrary)))
    (else
      (Rendering|Material|SetScalarParameterValue "/Game/MegaJam/BloodDripping/PC_Blood.PC_Blood" "Blood" 0.0 :!class /Script/Engine.KismetMaterialLibrary))))

(event EventBeginPlay
  (Utilities|FlowControl|Delay 0.2)
  (bind _outactors (Actor|GetAllActorsOfClass "/Game/MegaJam/Decals/BP_BloodDecal.BP_BloodDecal_C"))
  (Variables|Default|SetBloodDecals _outactors)
  (bind _outactors_2 (Actor|GetAllActorsOfClass "/Game/MegaJam/BloodDripping/BP_BloodDrops.BP_BloodDrops_C"))
  (Variables|Default|SetBloodDrops _outactors_2)
  (CallFunction|SetHorrorModeActive false false))

(fn ConstructionScript)

(fn SetHorrorModeActive
  (params (IsActive :type Boolean) (HasToLerpPostProcess :type Boolean))
  (bind _playercharacter (Variables|Default|GetPlayerCharacter))
  (bind _audio (Variables|/Game/MegaJam/BP_FirstPersonCharacter.BP_FirstPersonCharacter_C|GetAudio _playercharacter))
  (bind _output_get (Variables|Default|SetIsHorrorMordeActive? IsActive))
  (for _array_element (Variables|Default|GetBloodDecals)
    (Rendering|SetActorHiddenInGame _array_element (not _output_get)))
  (for _array_element_2 (Variables|Default|GetBloodDrops)
    (Rendering|SetActorHiddenInGame _array_element_2 (not _output_get)))
  (if HasToLerpPostProcess
    (CallFunction|LerpPostProcess)
    (CallFunction|SetBloodPuddleActive (Variables|Default|GetIsHorrorMordeActive?))
    (else
      (Rendering|Material|SetScalarParameterValue "/Game/MegaJam/PostProcess/PC_Pixel.PC_Pixel" "Switch" (Math|Conversions|ToFloat(Boolean) (Variables|Default|GetIsHorrorMordeActive?)) :!class /Script/Engine.KismetMaterialLibrary)))
  (Default|TurnFlashlightonOff (Variables|Default|GetPlayerCharacter) (Variables|Default|GetIsHorrorMordeActive?))
  (if (Variables|Default|GetIsHorrorMordeActive?)
    (Components|Activation|Activate _audio false)
    (else
      (Components|Activation|Deactivate _audio))))

(fn RegisterAllActors
  (return false false false))

(fn SetHorrorPP
  (params (IsActive :type Boolean))
  (Rendering|Material|SetScalarParameterValue "/Game/MegaJam/PostProcess/PC_Pixel.PC_Pixel" "Switch" (Math|Conversions|ToFloat(Boolean) IsActive) :!class /Script/Engine.KismetMaterialLibrary))

(fn SetBloodActive
  (params (IsActive :type Boolean))
  (bind _returnvalue (not IsActive))
  (for _array_element (Variables|Default|GetBloodDecals)
    (Rendering|SetActorHiddenInGame _array_element _returnvalue))
  (for _array_element_2 (Variables|Default|GetBloodDrops)
    (Rendering|SetActorHiddenInGame _array_element_2 _returnvalue))
  (CallFunction|SetBloodPuddleActive IsActive))