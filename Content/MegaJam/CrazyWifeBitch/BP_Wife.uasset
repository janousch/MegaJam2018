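; BP_Wife is the horror enemy character that screams on spawn, chases the player and kills on close contact.
; Pawn sensing by sight or noise drives its AI controller to chase at running speed, while Tick faces the target and extends a kill box within range.
; It can open doors, teleporting to the door's arrow.
; Death ragdolls it with blood effects, animates a material parameter collection and loads FinalScene.
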(event OnSeePawn(PawnSensing)
  (params (Pawn :type Pawn%20Object%20Reference))
  (if (not (Variables|Default|GetisDead))
    (Default|ChasePlayer (Variables|Default|GetAIController) Pawn)
    (Variables|Default|SetPlayerPawn Pawn)
    (Variables|/Script/Engine.CharacterMovementComponent|SetMaxWalkSpeed (Variables|Character|GetCharacterMovement) (Variables|Default|GetRUNNING_SPEED))
    (Variables|Default|SetIsPlayerTarget true)))

(event OnHearNoise(PawnSensing)
  (params (Instigator :type Pawn%20Object%20Reference) (Location :type Vector%20%28by%20ref%29 :default "0, 0, 0") (Volume :type Float%20%28single-precision%29))
  (if (not (Variables|Default|GetisDead))
    (Default|ChasePlayer (Variables|Default|GetAIController) Instigator)
    (Variables|Default|SetPlayerPawn Instigator)
    (Variables|/Script/Engine.CharacterMovementComponent|SetMaxWalkSpeed (Variables|Character|GetCharacterMovement) (Variables|Default|GetRUNNING_SPEED))
    (Variables|Default|SetIsPlayerTarget true)))

(event OnComponentBeginOverlap(Box)
  (params (OverlappedComponent :type Primitive%20Component%20Object%20Reference) (OtherActor :type Actor%20Object%20Reference) (OtherComp :type Primitive%20Component%20Object%20Reference) (OtherBodyIndex :type Integer) (bFromSweep :type Boolean) (SweepResult :type Hit%20Result%20Structure%20%28by%20ref%29))
  (Utilities|Behaviour
    (:CanKillAndChase
      (bind _asbp_first_person_character (Utilities|Casting|CastToBP_FirstPersonCharacter OtherActor))
      (Utilities|FlowControl|Delay 0.2)
      (Default|Die _asbp_first_person_character))))

(event Custom|CheckDoor
  (params (DoorReference :type Door%20Object%20Reference))
  (bind _arrow (Variables|/Game/MegaJam/Door/Door.Door_C|GetArrow DoorReference))
  (bind _returnvalue (Transformation|GetWorldTransform _arrow))
  (Utilities|IsValid DoorReference
    (:Is%20Valid
      (if (not (Utilities|Enum|Equal(Enum) (Variables|/Game/MegaJam/Door/Door.Door_C|GetDoorState DoorReference) "NewEnumerator2"))
        (Utilities|FlowControl|DoOnce false
          (:Completed
            (Default|OpentheDoor DoorReference)
            (Utilities|FlowControl|Delay 1.5)
            (Variables|/Game/MegaJam/Door/Door.Door_C|SetDoorState DoorReference "NewEnumerator5")
            (Utilities|IsValid self
              (:Is%20Valid
                (Transformation|SetActorTransform (Math|Transform|MakeTransform (Math|Vector|MakeVector (.x (.location _returnvalue)) (.y (.location _returnvalue)) (.z (Transformation|GetActorLocation))) (.rotation _returnvalue) "1,1,1"))))))))))

(event Custom|Death
  (bind _mesh (Variables|Character|GetMesh))
  (CallFunction|SetHorrorPPActive false)
  (Variables|Default|SetisDead true)
  (Default|StopMoving (Variables|Default|GetAIController))
  (Audio|Components|Audio|Stop (Variables|Default|GetAudio))
  (Collision|SetCollisionProfileName _mesh "BlockAll" :!class /Script/Engine.PrimitiveComponent)
  (Physics|SetSimulatePhysics _mesh true)
  (CallFunction|PlaySoundWife "/Game/MegaJam/Sounds/body_fall_1_Cue.body_fall_1_Cue" (CallFunction|BODYFALL))
  (Utilities|FlowControl|Delay 1.0)
  (Development|SetHiddeninGame (Variables|Default|GetDecalBlood) false false)
  (Components|Activation|Activate (Variables|Default|GetParticleBlood) false)
  (bind _newtrack_0 (Timeline|TL_Death Play)
    (:Update
      (Rendering|Material|SetScalarParameterValue "/Game/MegaJam/CrazyWifeBitch/PC_WifeDeath.PC_WifeDeath" "Death" _newtrack_0 :!class /Script/Engine.KismetMaterialLibrary))
    (:Finished
      (Utilities|FlowControl|Delay 3.0)
      (Game|OpenLevel(byName) "FinalScene"))))

(event Custom|StartChasingPlayer
  (params (PlayerCharacter :type BP%20First%20Person%20Character%20Object%20Reference))
  (bind _output_get (Variables|Default|SetPlayerPawn PlayerCharacter))
  (Utilities|Behaviour
    (:CanKillAndChase
      _)
    (:CanChase
      _))
  (Default|ChasePlayer (Variables|Default|GetAIController) _output_get)
  (Variables|/Script/Engine.CharacterMovementComponent|SetMaxWalkSpeed (Variables|Character|GetCharacterMovement) (Variables|Default|GetRUNNING_SPEED))
  (Variables|Default|SetIsPlayerTarget true))

(event Custom|StopChasingPlayer
  (Default|StopMoving (Variables|Default|GetAIController)))

(event EventBeginPlay
  (bind _audio (Variables|Default|GetAudio))
  (bind _asbp_aicontroller_wife (Utilities|Casting|CastToBP_AIControllerWife (Pawn|GetController)))
  (Variables|Default|SetAIController _asbp_aicontroller_wife)
  (Variables|/Game/MegaJam/BP_GameState.BP_GameState_C|SetWife (CallFunction|GetBPGameState) self)
  (Audio|Components|Audio|SetSound _audio "/Game/MegaJam/Sounds/scream_1_Cue.scream_1_Cue")
  (Audio|Components|Audio|Play _audio 0.0)
  (Default|Tension (CallFunction|GetPlayerCharacter)))

(event EventTick
  (params (DeltaSeconds :type Float%20%28single-precision%29))
  (bind _playerpawn (Variables|Default|GetPlayerPawn))
  (bind _returnvalue (Transformation|GetActorLocation _playerpawn))
  (if (Variables|Default|GetIsPlayerTarget)
    (Transformation|SetActorRotation (Math|Rotator|MakeRotator 0.0 0.0 (.yaw (Math|Rotator|FindLookatRotation (Transformation|GetActorLocation) _returnvalue))))
    (Variables|Default|SetLastLocation "0, 0, 0")
    (Utilities|IsValid _playerpawn
      (:Is%20Valid
        (bind _output_get (Variables|Default|SetCanKillPlayer (< (Math|Vector|VectorLength (- _returnvalue (Transformation|GetActorLocation))) 1e+02)))
        (Transformation|SetRelativeLocation (Variables|Default|GetBox) (Math|Vector|MakeVector (Math|Float|Lerp -24.0 6e+01 (Math|Conversions|ToFloat(Boolean) _output_get)) 0.0 0.0) false false)))))

(fn ConstructionScript)

(fn PlaySoundWife
  (params (NewSound :type Sound%20Base%20Object%20Reference) (VolumeMultiplier :type Float%20%28single-precision%29))
  (bind _audio (Variables|Default|GetAudio))
  (Audio|Components|Audio|SetSound _audio NewSound)
  (Audio|Components|Audio|SetVolumeMultiplier _audio VolumeMultiplier :!class /Script/Engine.AudioComponent))